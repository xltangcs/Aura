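; Player controller Blueprint for the Aura character that provides a dash ability.
; BeginPlay caches the character's movement component, camera and base values, and derives dash speed from timeline play rate times distance.
; Dash hides the pawn, disables input and boosts speed and acceleration while a timeline drives forward movement input and an FOV shift.
; When the timeline finishes, DashSetting restores base movement and visibility, and input is re-enabled.
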(event EventBeginPlay
  (bind _dashtimelineplayrate (Variables|Default|GetDashTimelinePlayRate))
  (bind _ascharacter (Utilities|Casting|CastToCharacter (Game|Player|GetPlayerPawn 0)))
  (Variables|Default|SetAuraCharacter _ascharacter)
  (bind _ascharacter_movement_component (Utilities|Casting|CastToCharacterMovementComponent (Pawn|GetMovementComponent (Variables|Default|GetAuraCharacter))))
  (bind _output_get (Variables|Default|SetAuraMovementComponent _ascharacter_movement_component))
  (Variables|Default|SetBaseAcceleration (Variables|/Script/Engine.CharacterMovementComponent|GetMaxAcceleration _output_get))
  (Variables|Default|SetBaseWalkSpeed (Variables|/Script/Engine.CharacterMovementComponent|GetMaxWalkSpeed _output_get))
  (Components|Timeline|SetPlayRate (Variables|Default|GetDashTimeline) _dashtimelineplayrate)
  (Variables|Default|SetDashSpeed (* _dashtimelineplayrate (Variables|Default|GetDashDistacne)))
  (Variables|Default|SetAuraCamera (Actor|GetComponentbyClass (Variables|Default|GetAuraCharacter) "/Script/Engine.CameraComponent"))
  (Variables|Default|SetBaseFov (Variables|/Script/Engine.CameraComponent|GetFieldOfView (Variables|Default|GetAuraCamera))))

(event EventTick
  (params (DeltaSeconds :type Float%20%28single-precision%29)))

(event EventDash
  (params (InputActionValue :type Input%20Action%20Value%20Structure%20%28by%20ref%29))
  (bind _returnvalue (Game|Player|GetPlayerPawn 0))
  (bind _basefov (Variables|Default|GetBaseFov))
  (CallFunction|DashSetting (Variables|Default|GetDashSpeed) 1e+05 true)
  (Input|DisableInput 0)
  (bind _newtrack_0 (Timeline|DashTimeline PlayFromStart)
    (:Update
      (Pawn|Input|AddMovementInput _returnvalue (Transformation|GetActorForwardVector _returnvalue) 1.0 false)
      (Camera|SetFieldOfView (Variables|Default|GetAuraCamera) (Math|Float|Lerp _basefov (+ _basefov 2e+01) _newtrack_0)))
    (:Finished
      ;[1 1 1] Finish
      (CallFunction|DashSetting (Variables|Default|GetBaseWalkSpeed) (Variables|Default|GetBaseAcceleration) false)
      (Input|EnableInput 0))))

(fn ConstructionScript)

(fn DashSetting
  (params (WalkSpeed :type Float%20%28double-precision%29) (Acceleration :type Float%20%28double-precision%29) (bIsHideActor :type Boolean))
  (bind _auramovementcomponent (Variables|Default|GetAuraMovementComponent))
  (Variables|/Script/Engine.CharacterMovementComponent|SetMaxWalkSpeed _auramovementcomponent WalkSpeed)
  (Variables|/Script/Engine.CharacterMovementComponent|SetMaxAcceleration _auramovementcomponent Acceleration)
  (Rendering|SetActorHiddenInGame (Game|Player|GetPlayerPawn 0) bIsHideActor))